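; GA_Jump is a Gameplay Ability that makes the player's humanoid character jump.
; On activation it checks the ability cost, then casts the avatar actor to DPlayerState and reaches the DHumanoidCharacter through its pawn.
; It calls the character's Jump, commits the cost and ends.
; It also ends when the cost check fails, but not when a cast or pawn validity check fails.
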(event `self.K2_ActivateAbility`
  (bind _returnvalue (`self.K2_CheckAbilityCost`))
  (if _returnvalue
    (bind _asdplayer_state (cast `DPlayerState` (`self.GetAvatarActorFromActorInfo`)))
    (bind _returnvalue_2 (`PlayerState.GetPawn` _asdplayer_state))
    (`/Engine/EditorBlueprintResources/StandardMacros.IsValid` _returnvalue_2
      (:`Is Valid`
        (bind _asdhumanoid_character (cast `DHumanoidCharacter` _returnvalue_2))
        (`Character.Jump` _asdhumanoid_character)
        (`self.K2_CommitAbilityCost` false)
        (`self.K2_EndAbility`)))
    (else
      (`self.K2_EndAbility`))))